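; Player controller that handles the attack input and blocks attack spamming through an IsAttacking flag.
; ServerAttack gets the montage from the controlled character's BP_CombatComponent, plays it, and passes it to MulticastPlayMontage for clients.
; The montage-ended callback clears the flag to allow the next attack.
; A debug input prints the player index returned by GetMyPlayerIndex.
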(event Custom|ServerAttack
  (if (not (Variables|Default|GetbIsAttacking))
    (Variables|Default|SetbIsAttacking true)
    ;[1 1 1] If the owned pawn has a combat component, get the current attack anim montage and play it
    (bind _ascharacter (Utilities|Casting|CastToCharacter (Pawn|GetControlledPawn)))
    (bind _attackanim (Default|GetAttackAnim (Actor|GetComponentbyClass _ascharacter "/Game/Blueprints/Combat/BP_CombatComponent.BP_CombatComponent_C")))
    (Utilities|IsValid _attackanim
      (:Is%20Valid
        (Animation|Montage|MontagePlay (Components|SkeletalMesh|GetAnimInstance (Variables|/Script/Engine.Character|GetMesh _ascharacter)) _attackanim 1.0 "MontageLength" 0.0 true)
        ;[1 1 1] When the montage is done, we can attack again
        (EventDispatchers|BindEventtoOnMontageEnded (Components|SkeletalMesh|GetAnimInstance (Variables|/Script/Engine.Character|GetMesh _ascharacter)) (delegate Custom|AttackFinished))
        ;[1 1 1] Play montage on all clients
        (CallFunction|MulticastPlayMontage _attackanim)))))

(event Custom|AttackFinished
  (params (Montage :type Anim%20Montage%20Object%20Reference) (bInterrupted :type Boolean))
  ;[1 1 1] When the montage is done, we can attack again
  (Variables|Default|SetbIsAttacking false))

(event Custom|MulticastPlayMontage
  (params (Montage :type Anim%20Montage%20Object%20Reference))
  ;[1 1 1] Play montage on clients
  (bind _ascharacter (Utilities|Casting|CastToCharacter (Pawn|GetControlledPawn)))
  (Animation|Montage|MontagePlay (Components|SkeletalMesh|GetAnimInstance (Variables|/Script/Engine.Character|GetMesh _ascharacter)) Montage 1.0 "MontageLength" 0.0 true))

(event Input|ActionEvents|InputActionAttack
  (params (Key :type Key%20Structure))
  ;[1 1 1] Don't allow spamming attack button. Server handles actual attack.
  (:Pressed
    (if (not (Variables|Default|GetbIsAttacking))
      (CallFunction|ServerAttack))))

(event Input|ActionEvents|InputActionDEBUG_PlayerInfo
  (params (Key :type Key%20Structure))
  (:Pressed
    (bind _playerindex (Class|TurnBasedBlueprintLibrary|GetMyPlayerIndex (Game|GetPlayerController 0)))
    (Development|PrintString (Utilities|String|BuildString(Integer) "" "" _playerindex))))

(fn ConstructionScript)