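; A combat dummy that shows its health as in-world text and visibly reacts when it takes damage.
; BP_HealthComponent events drive it: damage triggers a multicast reaction, and replicated health changes refresh the current/max text.
; The reaction plays the DamageBump timeline, offsetting the mesh in proportion to damage and flashing the color of a dynamic material created at BeginPlay.
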(event OnDamaged(BP_HealthComponent)
  (params (Damage :type Integer))
  ;[1 1 1] When the server notifies we are damaged, play a visual effect on all clients
  (CallFunction|MulticastDamageReact Damage))

(event OnHealthChanged(BP_HealthComponent)
  ;[1 1 1] When a change to our health is passed from the server via repnotify, update our damage text
  (CallFunction|UpdateDamageText))

(event Custom|MulticastDamageReact
  (params (Damage :type Integer))
  ;[1 1 1] When the server notifies we are damaged, play a visual effect on all clients
  (bind (_direction _location _colorflash) (Timeline|DamageBump PlayFromStart)
    (:Update
      (Transformation|SetRelativeLocation (Variables|Default|GetStaticMesh) (* _location Damage) false false)
      (Rendering|Material|SetVectorParameterValue (Variables|Default|GetDynamicMaterial) "Color" _colorflash :!class /Script/Engine.MaterialInstanceDynamic))))

(event EventBeginPlay
  (CallFunction|UpdateDamageText)
  (bind _returnvalue (Rendering|Material|CreateDynamicMaterialInstance (Variables|Default|GetStaticMesh) 0 "/Game/ExternalPacks/StarterContent/Materials/M_Basic_Wall.M_Basic_Wall" "None" :!class /Script/Engine.PrimitiveComponent))
  (Variables|Default|SetDynamicMaterial _returnvalue))

(fn ConstructionScript)

(fn UpdateDamageText
  (bind _bp_healthcomponent (Variables|Default|GetBP_HealthComponent))
  (Rendering|Components|TextRender|SetText (Variables|Default|GetTextRender) (Utilities|Text|FormatText "{health}/{max}" (Variables|/Game/Blueprints/Combat/BP_HealthComponent.BP_HealthComponent_C|GetCurrentHealth _bp_healthcomponent) (Variables|/Game/Blueprints/Combat/BP_HealthComponent.BP_HealthComponent_C|GetMaxHealth _bp_healthcomponent))))