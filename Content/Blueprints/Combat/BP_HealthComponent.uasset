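; Health component that tracks an actor's current health and broadcasts damage, death and health-change events.
; TakeDamage subtracts damage and fires OnDamaged, or sets health to zero and fires OnKilled before OnDamaged, with no guard against repeat kills.
; CurrentHealth uses a RepNotify to broadcast OnHealthChanged, while the MaxHealth RepNotify is empty.
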(event EventBeginPlay)

(event EventTick
  (params (DeltaSeconds :type Float%20%28single-precision%29)))

(fn TakeDamage
  (params (Damage :type Integer))
  (bind _output_get (LocalVariables|SetNewHealth (- (Variables|Default|GetCurrentHealth) Damage)))
  (if (> _output_get 0)
    (Variables|Default|SetCurrentHealth (LocalVariables|GetNewHealth))
    (Default|CallOnDamaged Damage)
    (else
      (Variables|Default|SetCurrentHealth 0)
      (Default|CallOnKilled)
      (Default|CallOnDamaged Damage))))

(fn OnRepCurrentHealth
  (Default|CallOnHealthChanged))

(fn OnRepMaxHealth)