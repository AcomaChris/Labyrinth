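; BP_CharacterManager is a debug actor that lets the player swap between the third-person character and the Minotaur boss.
; On the DEBUG_CharacterSwap input, it unpossesses and destroys the current pawn, spawns the other class at the same transform and has player controller 0 possess it.
; An IsBoss flag tracks which form is active so each press toggles between the two.
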(event EventBeginPlay)

(event Collision|EventActorBeginOverlap
  (params (OtherActor :type Actor%20Object%20Reference)))

(event EventTick
  (params (DeltaSeconds :type Float%20%28single-precision%29)))

(event Input|ActionEvents|InputActionDEBUG_CharacterSwap
  (params (Key :type Key%20Structure))
  (:Pressed
    (CallFunction|DEBUGSwapCharactertoBoss)))

(fn ConstructionScript)

(fn DEBUGSwapCharactertoBoss
  (bind _returnvalue (Game|GetPlayerController 0))
  (bind _returnvalue_2 (Game|GetPlayerController 0))
  (bind _output_get (LocalVariables|SetCurrentPawn (Pawn|GetControlledPawn _returnvalue_2)))
  (LocalVariables|SetCurrentTransform (Transformation|GetActorTransform _output_get))
  (Pawn|UnPossess _returnvalue_2)
  (Actor|DestroyActor (LocalVariables|GetCurrentPawn))
  (if (Variables|Default|GetIsBoss)
    (bind _returnvalue_3 (Game|SpawnActorfromClass "/Game/Characters/ThirdPersonCharacter.ThirdPersonCharacter_C" (LocalVariables|GetCurrentTransform) "Undefined" 0 0))
    (Variables|Default|SetIsBoss false)
    (Pawn|Possess _returnvalue _returnvalue_3)
    (else
      (bind _returnvalue_4 (Game|SpawnActorfromClass "/Game/Characters/Monster_Boss_Minotaur01.Monster_Boss_Minotaur01_C" (LocalVariables|GetCurrentTransform) "Undefined" 0 0))
      (Variables|Default|SetIsBoss true)
      (Pawn|Possess _returnvalue _returnvalue_4))))