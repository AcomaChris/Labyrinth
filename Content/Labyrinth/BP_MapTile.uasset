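; BP_MapTile is a labyrinth tile actor that randomizes its loot and wall openings in its construction script.
; A random roll against LootChance decides whether the Loot component and its children stay or are destroyed.
; For each N, S, E and W connection flagged in TileData, it casts that side's child actor to BP_DungeonWall.
; CreateConnection then randomly turns that wall into a door or destroys it.
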(event EventBeginPlay)

(event Collision|EventActorBeginOverlap
  (params (OtherActor :type Actor%20Object%20Reference)))

(event EventTick
  (params (DeltaSeconds :type Float%20%28single-precision%29)))

(fn ConstructionScript
  (bind _tiledata (Variables|Default|GetTileData))
  (bind (_n _s _e _w) (Utilities|Struct|BreakTile _tiledata))
  (Utilities|FlowControl|Sequence
    (:then_0
      (if (not (<= (Math|Random|RandomFloatinRange 0.0 1.0) (Variables|Default|GetLootChance)))
        (for _array_element (Components|GetChildrenComponents (Variables|Default|GetLoot) true)
          (Components|DestroyComponent _array_element))
        (Components|DestroyComponent (Variables|Default|GetLoot))))
    (:then_1
      (Utilities|FlowControl|Sequence
        (:then_0
          (if _n
            (bind _asbp_dungeon_wall (Utilities|Casting|CastToBP_DungeonWall (Variables|/Script/Engine.ChildActorComponent|GetChildActor (Variables|Default|GetNorthWall))))
            (CallFunction|CreateConnection _asbp_dungeon_wall)))
        (:then_1
          (if _s
            (bind _asbp_dungeon_wall_2 (Utilities|Casting|CastToBP_DungeonWall (Variables|/Script/Engine.ChildActorComponent|GetChildActor (Variables|Default|GetSouthWall))))
            (CallFunction|CreateConnection _asbp_dungeon_wall_2)))
        (:then_2
          (if _e
            (bind _asbp_dungeon_wall_3 (Utilities|Casting|CastToBP_DungeonWall (Variables|/Script/Engine.ChildActorComponent|GetChildActor (Variables|Default|GetEastWall))))
            (CallFunction|CreateConnection _asbp_dungeon_wall_3)))
        (:then_3
          (if _w
            (bind _asbp_dungeon_wall_4 (Utilities|Casting|CastToBP_DungeonWall (Variables|/Script/Engine.ChildActorComponent|GetChildActor (Variables|Default|GetWestWall))))
            (CallFunction|CreateConnection _asbp_dungeon_wall_4)))))))

(fn CreateConnection
  (params (Wall :type BP%20Dungeon%20Wall%20Object%20Reference))
  (switch int (Math|Random|RandomIntegerinRange 0 1)
    (:Default
      (Actor|DestroyActor Wall :!label _label))
    (:0
      (Default|MakeDoor Wall))
    (:1
      (goto _label))))