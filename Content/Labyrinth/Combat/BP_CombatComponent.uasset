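; Combat component that resolves weapon hits and supplies attack animations for the current weapon in the Labyrinth game.
; SetWeapon caches damage from DT_Weapons, and GetAttackAnim reads the animation from the same table, falling back to DefaultAttack.
; HandleWeaponOverlap damages non-owner actors that have a BP_HealthComponent while Attacking is set, tracking HitActors so each is hit once per attack.
; EndAttack clears the attack flag and hit list.
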(event EventBeginPlay)

(event EventTick
  (params (DeltaSeconds :type Float%20%28single-precision%29)))

(fn GetAttackAnim
  (bind _returnvalue (Utilities|GetDataTableRow "/Game/Labyrinth/Combat/Weapons/DT_Weapons.DT_Weapons" (Variables|Default|GetCurrentWeapon))
    (:then
      (return (.AttackAnim (Utilities|Struct|BreakS_Weapon _returnvalue))))
    (:RowNotFound
      (return (Variables|Default|GetDefaultAttack)))))

(fn HandleWeaponOverlap
  (params (HitActor :type Actor%20Object%20Reference))
  (bind _returnvalue (Actor|GetComponentbyClass HitActor "/Game/Labyrinth/Combat/BP_HealthComponent.BP_HealthComponent_C"))
  (if (!= HitActor (Components|GetOwner))
    (if (Variables|Default|GetAttacking)
      (if (not (Utilities|Array|ContainsItem (Variables|Default|GetHitActors) HitActor))
        (Utilities|IsValid _returnvalue
          (:Is%20Valid
            (Default|TakeDamage _returnvalue (Variables|Default|GetWeaponDamage))
            (Utilities|Array|Add (Variables|Default|GetHitActors) HitActor)))))))

(fn EndAttack
  (Variables|Default|SetAttacking false)
  (Utilities|Array|Clear (Variables|Default|GetHitActors)))

(fn SetWeapon
  (params (WeaponName :type Name))
  (bind _output_get (Variables|Default|SetCurrentWeapon WeaponName))
  (bind _returnvalue (Utilities|GetDataTableRow "/Game/Labyrinth/Combat/Weapons/DT_Weapons.DT_Weapons" _output_get)
    (:then
      (Variables|Default|SetWeaponDamage (Utilities|Struct|BreakS_Weapon _returnvalue)))))