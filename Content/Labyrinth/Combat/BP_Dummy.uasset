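; BP_Dummy is a combat dummy in the Labyrinth game that displays its health as text in the world.
; It binds a handler to the damage event of its BPHealthComponent on BeginPlay.
; A shared UpdateDamageText function writes current and maximum health to a TextRender component, both at start and whenever damage is reported, so no Tick is used.
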(event Custom|Damaged
  (CallFunction|UpdateDamageText))

(event EventBeginPlay
  (CallFunction|UpdateDamageText)
  (EventDispatchers|BindEventtoOnDamaged (Variables|Default|GetBP_HealthComponent) (delegate Custom|Damaged)))

(fn ConstructionScript)

(fn UpdateDamageText
  (bind _bp_healthcomponent (Variables|Default|GetBP_HealthComponent))
  (Rendering|Components|TextRender|SetText (Variables|Default|GetTextRender) (Utilities|Text|FormatText "{health}/{max}" (Variables|/Game/Labyrinth/Combat/BP_HealthComponent.BP_HealthComponent_C|GetCurrentHealth _bp_healthcomponent) (Variables|/Game/Labyrinth/Combat/BP_HealthComponent.BP_HealthComponent_C|GetMaxHealth _bp_healthcomponent))))