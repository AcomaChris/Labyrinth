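; Lootable weapon pickup that becomes a random weapon from DT_Weapons at BeginPlay and takes that row's static mesh.
; On overlap, it sends the weapon's row name to the other actor through EquipWeaponMessage.
; A successful equip removes the mesh, stops the swirl effect and plays flash and short pickup effects, destroying the actor when the short effect finishes.
; A failed equip only prints a debug message.
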(event OnComponentBeginOverlap(PickupCollider)
  (params (OverlappedComponent :type Primitive%20Component%20Object%20Reference) (OtherActor :type Actor%20Object%20Reference) (OtherComp :type Primitive%20Component%20Object%20Reference) (OtherBodyIndex :type Integer) (bFromSweep :type Boolean) (SweepResult :type Hit%20Result%20Structure%20%28by%20ref%29))
  (bind _weapontype (Variables|Default|GetWeaponType))
  (bind _success (Class|BPIArmable|EquipWeapon(Message) OtherActor _weapontype))
  (Development|PrintString (Utilities|String|ToString(Name) _weapontype))
  (if _success
    (EventDispatchers|BindEventtoOnSystemFinished (Variables|Default|GetPickupShort) (delegate Custom|Done))
    (Components|Activation|Activate (Variables|Default|GetPickupFlash) true)
    (Components|DestroyComponent (Variables|Default|GetWeaponMesh))
    (Components|Activation|Activate (Variables|Default|GetPickupShort) true)
    (Components|Activation|Deactivate (Variables|Default|GetPickupConstantSwirl))
    (else
      (Development|PrintString "Was not able to equip weapon"))))

(event Custom|Done
  (params (PSystem :type Particle%20System%20Component%20Object%20Reference))
  (Actor|DestroyActor))

(event EventBeginPlay
  (bind _outrownames (DataTable|GetDataTableRowNames "/Game/Labyrinth/Combat/DT_Weapons.DT_Weapons"))
  (bind _output_get (Variables|Default|SetWeaponType (Utilities|Array|Get(acopy) _outrownames (- (Math|Random|RandomIntegerinRange 1 (Utilities|Array|Length _outrownames)) 1))))
  (bind _returnvalue (Utilities|GetDataTableRow "/Game/Labyrinth/Combat/DT_Weapons.DT_Weapons" _output_get)
    (:then
      (Components|StaticMesh|SetStaticMesh (Variables|Default|GetWeaponMesh) (.StaticMesh (Utilities|Struct|BreakS_Weapon _returnvalue))))))

(fn ConstructionScript)