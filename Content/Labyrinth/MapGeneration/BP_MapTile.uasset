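; BP_MapTile is a labyrinth map tile that assembles its walls and optional loot in the Construction Script.
; A random roll against LootChance keeps or destroys the Loot component and its children.
; TileData's N/S/E/W flags drive CreateWall, which sets each wall's child actor to BP_DungeonWall, or for passages randomly to BP_DungeonPassage or leaves it unchanged.
; The randomisation is noted as not yet multiplayer friendly.
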(event EventBeginPlay)

(event Collision|EventActorBeginOverlap
  (params (OtherActor :type Actor%20Object%20Reference)))

(event EventTick
  (params (DeltaSeconds :type Float%20%28single-precision%29)))

(fn ConstructionScript
  (bind _tiledata (Variables|Default|GetTileData))
  (bind (_n _s _e _w) (Utilities|Struct|BreakTile _tiledata))
  ;[1 1 1] Not made multiplayer friendly yet!
  (Utilities|FlowControl|Sequence
    (:then_0
      (if (not (<= (Math|Random|RandomFloatinRange 0.0 1.0) (Variables|Default|GetLootChance)))
        (for _array_element (Components|GetChildrenComponents (Variables|Default|GetLoot) true)
          (Components|DestroyComponent _array_element))
        (Components|DestroyComponent (Variables|Default|GetLoot))))
    (:then_1
      (Utilities|FlowControl|Sequence
        (:then_0
          (CallFunction|CreateWall _n (Variables|Default|GetNorthWall)))
        (:then_1
          (CallFunction|CreateWall _s (Variables|Default|GetSouthWall)))
        (:then_2
          (CallFunction|CreateWall _e (Variables|Default|GetEastWall)))
        (:then_3
          (CallFunction|CreateWall _w (Variables|Default|GetWestWall)))))))

(fn CreateWall
  (params (IsPassage :type Boolean) (WallComponent :type Child%20Actor%20Component%20Object%20Reference))
  (if IsPassage
    (switch int (Math|Random|RandomIntegerinRange 0 1) ; 50/50 door or blank
      (:0
        (ChildActorComponent|SetChildActorClass WallComponent "/Game/Labyrinth/MapGeneration/BP_DungeonPassage.BP_DungeonPassage_C")))
    (else
      (ChildActorComponent|SetChildActorClass WallComponent "/Game/Labyrinth/MapGeneration/BP_DungeonWall.BP_DungeonWall_C"))))