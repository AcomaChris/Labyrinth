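; BP_MapGenerator is an actor that builds the labyrinth map as a grid of tiles when play begins.
; On the authority only, it calls GenerateMap with the map dimensions, then walks the nested Map array and spawns a BP_MapTile per cell, passing in that cell's tile data.
; GetTileTransform offsets each tile from the actor's location along world X by column and Y by row, copying the actor's rotation and scale.
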(event EventBeginPlay
  (Networking|SwitchHasAuthority
    (:Authority
      (Class|MapGenerator|GenerateMap (Variables|Default|GetMapHeight) (Variables|Default|GetMapWidth))
      (for (_array_element _array_index) (Variables|Default|GetMap)
        (for (_array_element_2 _array_index_2) (Utilities|Struct|BreakTile2DArray _array_element)
          (bind _returnvalue (CallFunction|GetTileTransform _array_index _array_index_2))
          (Game|SpawnActorfromClass "/Game/Labyrinth/MapGeneration/BP_MapTile.BP_MapTile_C" _returnvalue "Undefined" 0 _array_element_2 0))))))

(fn ConstructionScript)

(fn GetTileTransform
  (params (Row :type Integer) (Column :type Integer))
  (bind _returnvalue (Transformation|GetActorTransform))
  (bind (_location _rotation _scale) (Math|Transform|BreakTransform _returnvalue))
  (return (Math|Transform|MakeTransform (+ (Math|Vector|MakeVector (Math|Conversions|ToFloat(Integer) (* Column (Variables|Default|GetTileWidth))) 0.0 0.0) (+ (Math|Vector|MakeVector 0.0 (Math|Conversions|ToFloat(Integer) (* Row (Variables|Default|GetTileHeight))) 0.0) _location)) _rotation _scale)))