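; BP_DungeonWall is a labyrinth wall piece that varies its look and can be turned into a door.
; Its Construction Script randomly either swaps the wall mesh to decorative arches or removes the torch.
; MakeDoor destroys the wall component with all its child components, then makes the door component visible.
; The event graph holds only disabled placeholder events.
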(event EventBeginPlay)

(event Collision|EventActorBeginOverlap
  (params (OtherActor :type Actor%20Object%20Reference)))

(event EventTick
  (params (DeltaSeconds :type Float%20%28single-precision%29)))

(fn ConstructionScript
  (switch int (Math|Random|RandomIntegerinRange 0 1)
    (:0
      (Components|StaticMesh|SetStaticMesh (Variables|Default|GetWall) "/Game/MedievalDungeon/Meshes/Architecture/Dungeon/SM_Decorative_Arches.SM_Decorative_Arches"))
    (:1
      (Components|DestroyComponent (Variables|Default|GetTorch)))))

(fn MakeDoor
  (for _array_element (Components|GetChildrenComponents (Variables|Default|GetWall) true)
    (Components|DestroyComponent _array_element))
  (Components|DestroyComponent (Variables|Default|GetWall))
  (Rendering|SetVisibility (Variables|Default|GetDoor) true false))